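; Arena game mode Blueprint that owns the player HUD and the match's music and end-of-game audio.
; BeginPlay creates the player widget, which the card selection events open with the card component's data or close.
; StartGame spawns background music and keeps the reference.
; FinishGame fades that music out if still valid, waits out the fade, then plays a win or fail sound based on arena game state.
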(event `self.ReceiveBeginPlay`
  (bind _returnvalue (`|CreateWidget` "/Game/Blueprints/Widgets/WBP_PlayerWidget.WBP_PlayerWidget_C"))
  (bind _output_get (set `self.PlayerUI` _returnvalue))
  (`UserWidget.AddToViewport` _output_get 0))

(event `self.StartGame`
  (bind _returnvalue (`GameplayStatics.SpawnSound2D` (`self.BackgroundMusic`) 1.0 1.0 0.0 null))
  (set `self.BackgroundAudio` _returnvalue))

(event `self.FinishGame`
  (`self.HandleSound`))

(event `HandleSound`
  (bind _backgroundaudio (`self.BackgroundAudio`))
  (bind _fadeouttime (`self.FadeOutTime`))
  ;[0 0 0] End Game Sound
  (if (`KismetSystemLibrary.IsValid` _backgroundaudio)
    (`AudioComponent.FadeOut` _backgroundaudio _fadeouttime 0.0 "Linear")
    (`KismetSystemLibrary.Delay` _fadeouttime)
    (switch `EGameStates` (`self.GetArenaGameState`)
      (:`Lost`
        (`GameplayStatics.PlaySound2D` (`self.FailSound`) 1.0 1.0 0.0 null null))
      (:`Win`
        (`GameplayStatics.PlaySound2D` (`self.WinSound`) 1.0 1.0 0.0 null null)))))

(event `self.OpenCardSelectionUI`
  (`/Game/Blueprints/Widgets/WBP_PlayerWidget.OpenCardUI` (`self.PlayerUI`) (`CardManagementComponent.CardsData` (`self.GetCardComp`))))

(event `self.CloseCardSelectionUI`
  (`/Game/Blueprints/Widgets/WBP_PlayerWidget.CloseCardUI` (`self.PlayerUI`) :!label _label))

(event `CloseCardUI`
  (goto _label))

(fn `UserConstructionScript`)