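; BP_ProjectileBase_Sinus is a projectile Blueprint that explodes itself when the arena is in certain non-gameplay states.
; BeginPlay runs the parent logic and caches the arena game mode.
; Each Tick calls the parent, then checks the arena game state and calls Explode for states such as menu, pause, prepare, win or lost.
; No sine motion is defined here, and the overlap override is disabled.
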(event `self.ReceiveBeginPlay`
  (`parent.ReceiveBeginPlay`)
  (bind _asbp_arena_game_mode (cast `/Game/Blueprints/GameModes/BP_ArenaGameMode` (`GameplayStatics.GetGameMode`)))
  (set `self.As BP Arena Game Mode` _asbp_arena_game_mode))

(event `self.ReceiveTick`
  (params (DeltaSeconds :type "Float (single-precision)"))
  (`parent.ReceiveTick` DeltaSeconds)
  (switch `EGameStates` (`ArenaGameMode.GetArenaGameState` (`self.As BP Arena Game Mode`))
    (:`None`
      _)
    (:`Menu`
      _)
    (:`Ready`
      _)
    (:`Pause`
      _)
    (:`Lost`
      _)
    (:`Win`
      _)
    (:`Prepare`
      _))
  (`self.Explode`))

(fn `UserConstructionScript`
  (`parent.UserConstructionScript`))